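; BP_SpartaPlayerController is a player controller Blueprint with Enhanced Input events for jump, look, move, sprint and inventory.
; Only IA_Inventory does anything, printing debug text and its action value, with both branch paths printing the same thing.
; Disconnected logic would swap the IMC_Character and IMC_UI mapping contexts and set IsUIOpen, but it never runs.
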(event `EnhancedInput|/Game/Inputs/IA_Jump`
  (params (ActionValue :type Boolean) (ElapsedSeconds :type "Float (double-precision)") (TriggeredSeconds :type "Float (double-precision)") (InputAction :type "InputAction Object Reference" :default "/Game/Inputs/IA_Jump.IA_Jump")))

(event `EnhancedInput|/Game/Inputs/IA_Look`
  (params (ActionValue :type "Vector2D Structure") (ElapsedSeconds :type "Float (double-precision)") (TriggeredSeconds :type "Float (double-precision)") (InputAction :type "InputAction Object Reference" :default "/Game/Inputs/IA_Look.IA_Look")))

(event `EnhancedInput|/Game/Inputs/IA_Move`
  (params (ActionValue :type "Vector2D Structure") (ElapsedSeconds :type "Float (double-precision)") (TriggeredSeconds :type "Float (double-precision)") (InputAction :type "InputAction Object Reference" :default "/Game/Inputs/IA_Move.IA_Move")))

(event `EnhancedInput|/Game/Inputs/IA_Sprint`
  (params (ActionValue :type Boolean) (ElapsedSeconds :type "Float (double-precision)") (TriggeredSeconds :type "Float (double-precision)") (InputAction :type "InputAction Object Reference" :default "/Game/Inputs/IA_Sprint.IA_Sprint")))

(event `EnhancedInput|/Game/Inputs/IA_Inventory`
  (params (ActionValue :type Boolean) (ElapsedSeconds :type "Float (double-precision)") (TriggeredSeconds :type "Float (double-precision)") (InputAction :type "InputAction Object Reference" :default "/Game/Inputs/IA_Inventory.IA_Inventory"))
  (:`Triggered`
    (`KismetSystemLibrary.PrintString` "Tab")
    (if ActionValue
      (`KismetSystemLibrary.PrintString` (`KismetStringLibrary.Conv_BoolToString` ActionValue))
      (else
        (`KismetSystemLibrary.PrintString` (`KismetStringLibrary.Conv_BoolToString` ActionValue))))))

(fn `UserConstructionScript`)